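; BP_GI_NFT, by its name a game instance, provides helper functions for an access token and a server URL.
; GetServerURL appends a slash to ServerURL, and TestWindowsTokenFilePath builds an absolute path to Token.txt in the project's Saved directory.
; GetTokenByPlatform switches on the platform name but has no connected cases, leaving its empty-string return unreachable.
; SetAccessToken is an empty stub, so no token is read or stored here.
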(fn `Get Server URL`
  (returns (ServerURL :type String))
  (return (`KismetStringLibrary.Concat_StrStr` (`self.ServerURL`) "/")))

(fn `GetTokenByPlatform`
  (returns (Token :type String))
  (switch `string` (`GameplayStatics.GetPlatformName`)))

(fn `SetAccessToken`
  (params (NewToken :type String)))

(fn `TestWindowsTokenFilePath`
  (returns (ReturnValue :type String))
  (return (`KismetStringLibrary.Concat_StrStr` (`KismetSystemLibrary.ConvertToAbsolutePath` (`BlueprintPathsLibrary.ProjectSavedDir`)) "Token.txt")))